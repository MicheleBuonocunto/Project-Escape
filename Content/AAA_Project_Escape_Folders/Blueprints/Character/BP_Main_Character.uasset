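; Player character Blueprint for the Escape project, handling movement, camera look and interaction through Enhanced Input.
; BeginPlay adds the character mapping context; input actions drive controller yaw and pitch and movement along the actor's forward and right vectors.
; Interaction fires the DISPInteraction dispatcher when CanInteract is true, otherwise printing a placeholder failure message meant to become a sound.
; CanInteract is only read in these graphs, never set.
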(event Input|EnhancedActionEvents|EnhancedInputActionIA_Camera
  (params (ActionValue :type Vector%202D%20Structure) (ElapsedSeconds :type Float%20%28double-precision%29) (TriggeredSeconds :type Float%20%28double-precision%29) (InputAction :type Input%20Action%20Object%20Reference :default "/Game/AAA_Project_Escape_Folders/Blueprints/Character/Input/Input_Actions/IA_Camera.IA_Camera"))
  (bind (_x _y) (Math|Vector2D|BreakVector2D ActionValue))
  ;[1 1 1] Camera movement
  (:Triggered
    ;;[1 1 1] Left-right camera movement
    (Pawn|Input|AddControllerYawInput _x)
    ;;[1 1 1] Up-Down movemnt
    (Pawn|Input|AddControllerPitchInput _y)))

(event Input|EnhancedActionEvents|EnhancedInputActionIA_Movement
  (params (ActionValue :type Vector%202D%20Structure) (ElapsedSeconds :type Float%20%28double-precision%29) (TriggeredSeconds :type Float%20%28double-precision%29) (InputAction :type Input%20Action%20Object%20Reference :default "/Game/AAA_Project_Escape_Folders/Blueprints/Character/Input/Input_Actions/IA_Movement.IA_Movement"))
  (bind (_x _y) (Math|Vector2D|BreakVector2D ActionValue))
  ;[1 1 1] Movement
  (:Triggered
    ;;[1 1 1] LeftRight
    (Pawn|Input|AddMovementInput (Transformation|GetActorRightVector) _x false)
    ;;[1 1 1] FrontBack
    (Pawn|Input|AddMovementInput (Transformation|GetActorForwardVector) _y false)))

(event Input|EnhancedActionEvents|EnhancedInputActionIA_Interaction
  (params (ActionValue :type Boolean) (ElapsedSeconds :type Float%20%28double-precision%29) (TriggeredSeconds :type Float%20%28double-precision%29) (InputAction :type Input%20Action%20Object%20Reference :default "/Game/AAA_Project_Escape_Folders/Blueprints/Character/Input/Input_Actions/IA_Interaction.IA_Interaction"))
  (:Started
    (if (Variables|Default|GetCan%20Interact?)
      (Default|CallDISPInteraction)
      (else
        (Development|PrintString "Impossible interact (To replace with sound)" true true "(R=1.000000,G=0.026564,B=0.073003,A=1.000000)")))))

(event EventBeginPlay
  ;[1 1 1] Character begin play - Cast to the controller - Add the mapping context
  (bind _asplayer_controller (Utilities|Casting|CastToPlayerController (Pawn|GetController)))
  (Utilities|IsValid (PlayerController|LocalPlayerSubsystems|GetEnhancedInputLocalPlayerSubsystem _asplayer_controller)
    (:Is%20Valid
      (Input|AddMappingContext (PlayerController|LocalPlayerSubsystems|GetEnhancedInputLocalPlayerSubsystem _asplayer_controller) "/Game/AAA_Project_Escape_Folders/Blueprints/Character/Input/Input_Mapping_Context/IMC_Character.IMC_Character" 0 "(bIgnoreAllPressedKeysUntilRelease=True,bForceImmediately=False)"))))

(event Collision|EventActorBeginOverlap
  (params (OtherActor :type Actor%20Object%20Reference)))

(event EventTick
  (params (DeltaSeconds :type Float%20%28single-precision%29)))

(fn ConstructionScript)