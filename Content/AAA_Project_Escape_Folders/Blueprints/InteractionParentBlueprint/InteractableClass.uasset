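; InteractableClass is a base interactable Actor that lets the player trigger an interaction near it.
; Its Box trigger sets CanInteract on BP_Main_Character during overlap and clears it on exit.
; At BeginPlay it binds evActivate to the player character's DISPInteraction dispatcher, independent of overlap.
; Activation currently only prints debug text.
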(event OnComponentBeginOverlap(Box)
  (params (OverlappedComponent :type Primitive%20Component%20Object%20Reference) (OtherActor :type Actor%20Object%20Reference) (OtherComp :type Primitive%20Component%20Object%20Reference) (OtherBodyIndex :type Integer) (bFromSweep :type Boolean) (SweepResult :type Hit%20Result%20Structure%20%28by%20ref%29))
  ;[1 1 1] Control if player is in the collider and active the interaction
  (bind _asbp_main_character (Utilities|Casting|CastToBP_Main_Character OtherActor))
  (Development|PrintString "Interactable")
  (Variables|/Game/AAA_Project_Escape_Folders/Blueprints/Character/BP_Main_Character.BP_Main_Character_C|SetCan%20Interact? _asbp_main_character true))

(event OnComponentEndOverlap(Box)
  (params (OverlappedComponent :type Primitive%20Component%20Object%20Reference) (OtherActor :type Actor%20Object%20Reference) (OtherComp :type Primitive%20Component%20Object%20Reference) (OtherBodyIndex :type Integer))
  ;[1 1 1] Player exit from the trigger
  (bind _asbp_main_character (Utilities|Casting|CastToBP_Main_Character OtherActor))
  (Variables|/Game/AAA_Project_Escape_Folders/Blueprints/Character/BP_Main_Character.BP_Main_Character_C|SetCan%20Interact? _asbp_main_character false))

(event Custom|evActivate
  (Development|PrintString "Activate" true true "(R=0.139379,G=1.000000,B=0.255825,A=1.000000)"))

(event EventBeginPlay
  (bind _asbp_main_character (Utilities|Casting|CastToBP_Main_Character (Game|GetPlayerCharacter 0)))
  (EventDispatchers|BindEventtoDISPInteraction _asbp_main_character (delegate Custom|evActivate)))

(fn ConstructionScript)